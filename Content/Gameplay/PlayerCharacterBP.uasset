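; Player character Blueprint that gives the player a starting loadout of weapons and ammo.
; On BeginPlay, it creates an assault rifle, a pistol and matching ammo stacks through the CharacterInventory component's storage.
; Each created item goes into its own fixed storage slot, with data assets defining the item type and the construction script left empty.
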(event EventBeginPlay
  (bind _characterinventory (Variables|Default|GetCharacterInventory))
  (bind _storage (Variables|/Script/MPO.InventoryComponent|GetStorage _characterinventory))
  (Utilities|FlowControl|Sequence
    (:then_0
      (bind _returnvalue (Class|ItemStorage|CreateItem _storage "/Script/MPO.WeaponItem" "/Game/DataAssets/Weapons/AssaultRifle.AssaultRifle" 1))
      (Class|ItemStorage|SetCellContent _storage 0 _returnvalue))
    (:then_1
      (bind _returnvalue_2 (Class|ItemStorage|CreateItem _storage "/Script/MPO.WeaponItem" "/Game/DataAssets/Weapons/Pistol.Pistol" 1))
      (Class|ItemStorage|SetCellContent _storage 1 _returnvalue_2))
    (:then_2
      (bind _returnvalue_3 (Class|ItemStorage|CreateItem _storage "/Script/MPO.AmmoItem" "/Game/DataAssets/Ammo/AssaultRifleAmmo.AssaultRifleAmmo" 50))
      (Class|ItemStorage|SetCellContent _storage 2 _returnvalue_3))
    (:then_3
      (bind _returnvalue_4 (Class|ItemStorage|CreateItem _storage "/Script/MPO.AmmoItem" "/Game/DataAssets/Ammo/PistolAmmo.PistolAmmo" 50))
      (Class|ItemStorage|SetCellContent _storage 3 _returnvalue_4))))

(fn ConstructionScript)